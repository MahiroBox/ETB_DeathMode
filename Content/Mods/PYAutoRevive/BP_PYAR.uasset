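; PYAutoRevive mod Blueprint that revives spectating players, toggled or triggered through mod buttons for auto revive, revive self and revive all.
; GetPlayer finds controllers whose pawn is a BP_Spectator rather than a character, destroys that pawn and restarts the player through the GameMode.
; Tick runs auto revive across 16 player slots and, behind a one-second Delay, also resizes each MP_PS ItemsRep array to 24.
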(event `self.ReceiveTick`
  (params (DeltaSeconds :type "Float (single-precision)"))
  (`self.AutoRevive`)
  (`KismetSystemLibrary.Delay` 1.0)
  (for _index (range 16)
    (bind _asmp_ps (cast `/Game/Multiplayer/MP_PS` (`Controller.PlayerState` (`GameplayStatics.GetPlayerController` _index))))
    (`KismetArrayLibrary.Array_Resize` (`/Game/Multiplayer/MP_PS.Items_Rep` _asmp_ps) 24)))

(fn `AutoRevive`
  (if (`self.IsAutoRevive`)
    (for _index (range 16)
      (`self.GetPlayer` _index))))

(fn `GetPlayer`
  (params (PlayerIndex :type Integer))
  (bind _returnvalue (`GameplayStatics.GetPlayerController` PlayerIndex))
  (bind _returnvalue_2 (`GameplayStatics.GetPlayerPawn` PlayerIndex))
  (`/Engine/EditorBlueprintResources/StandardMacros.IsValid` _returnvalue_2
    (:`Is Valid`
      (`/Engine/EditorBlueprintResources/StandardMacros.IsValid` _returnvalue
        (:`Is Valid`
          (`/Engine/EditorBlueprintResources/StandardMacros.IsValid` (`GameplayStatics.GetPlayerCharacter` PlayerIndex)
            (:`Is Not Valid`
              (castclass `/Game/Game/BP_Spectator` (`GameplayStatics.GetObjectClass` _returnvalue_2))
              (`self.K2_DestroyActor` _returnvalue_2)
              (`GameModeBase.RestartPlayer` (`GameplayStatics.GetGameMode`) _returnvalue))))))))

(fn `ModButtonWasPressed`
  (params (FunctionIndex :type Integer))
  (locals (NewLocalVar_0 :type "Array of EObjectTypeQuery Enum"))
  (switch `int` FunctionIndex
    (:`0`
      (bind _output_get (set `self.IsAutoRevive` (not (stale _output_get))))
      (`/Game/Mods/Z_DebugLog_P/BlueprintLibraries/BFL_DebugLog.ModPrint` (`KismetStringLibrary.Concat_StrStr` "Auto Revive: " (`KismetStringLibrary.Conv_BoolToString` _output_get))))
    (:`1`
      (`self.ReviveSelf`))
    (:`2`
      (`self.ReviveAll`))))

(fn `ReviveAll`
  (for _index (range 16)
    (`self.GetPlayer` _index)))

(fn `ReviveSelf`
  (`self.GetPlayer` 0))

(fn `UserConstructionScript`
  (`parent.UserConstructionScript`))