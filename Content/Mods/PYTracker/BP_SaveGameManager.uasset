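; Save manager for the PYTracker mod that persists recorded tracks of transforms, velocities and map-related data.
; On BeginPlay it loads or creates a TrackerSave and records the level name if none is stored.
; Samples accumulate in a buffer, which replaces saved tracks or, in mix mode, appends to them, clearing on map change.
; It also resets saves and writes separate slots with custom or level-and-timestamp names.
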(event `self.ReceiveBeginPlay`
  (bind _trackersave (`self.TrackerSave`))
  (`self.CheckSave`)
  (if (`KismetStringLibrary.IsEmpty` (`/Game/Mods/PYTracker/Saves/TrackerSave.lastMap` _trackersave))
    (bind _returnvalue (`GameplayStatics.GetCurrentLevelName` true))
    (set `/Game/Mods/PYTracker/Saves/TrackerSave.lastMap` _returnvalue _trackersave)
    (`self.SaveObjectToSlot` false)))

(fn `AddToTrackerDummy`
  (params (Transforms :type "Transform Structure") (MapRelated :type String) (Velocity :type "Vector Structure"))
  (locals (NewArrays :type "Array of Transform Structure"))
  (bind (_transforms _velocity _maprelated) (break `/Game/Mods/PYTracker/Saves/S_TrackerDataList` (`self.StrackerDummy`)))
  (`KismetArrayLibrary.Array_Add` _maprelated MapRelated)
  (`KismetArrayLibrary.Array_Add` _transforms Transforms)
  (`KismetArrayLibrary.Array_Add` _velocity Velocity)
  (set `self.StrackerDummy` (make `/Game/Mods/PYTracker/Saves/S_TrackerDataList` _transforms _velocity _maprelated)))

(fn `CheckSave`
  (bind _returnvalue (`GameplayStatics.DoesSaveGameExist` (`self.SaveGameName`)))
  (if _returnvalue
    (bind _returnvalue_2 (`GameplayStatics.LoadGameFromSlot` (`self.SaveGameName`)))
    (bind _astracker_save (cast `/Game/Mods/PYTracker/Saves/TrackerSave` _returnvalue_2))
    (set `self.TrackerSave` _astracker_save)
    (else
      (bind _returnvalue_3 (`GameplayStatics.CreateSaveGameObject` "/Game/Mods/PYTracker/Saves/TrackerSave.TrackerSave_C"))
      (set `self.TrackerSave` _returnvalue_3))))

(fn `ResetSave`
  (params (isResetTrackerOnly :type Boolean))
  (if isResetTrackerOnly
    (`KismetArrayLibrary.Array_Clear` (`/Game/Mods/PYTracker/Saves/TrackerSave.S_TrackerDatas` (`self.TrackerSave`)))
    (`self.SaveObjectToSlot` false)
    (else
      (set `self.StrackerDummy` (struct))
      (bind _returnvalue (`GameplayStatics.CreateSaveGameObject` "/Game/Mods/PYTracker/Saves/TrackerSave.TrackerSave_C"))
      (bind _output_get (set `self.TrackerSave` _returnvalue))
      (`GameplayStatics.SaveGameToSlot` _output_get (`self.SaveGameName`)))))

(fn `SaveCurrentTrack`
  (bind _trackersave (`self.TrackerSave`))
  (bind _s_trackerdatas (`/Game/Mods/PYTracker/Saves/TrackerSave.S_TrackerDatas` (`self.TrackerSave`)))
  (if (`/Game/Mods/PYTracker/Saves/TrackerSave.isMixTrack` (`self.TrackerSave`))
    (bind _returnvalue (`GameplayStatics.GetCurrentLevelName` true))
    (if (`KismetStringLibrary.NotEqual_StrStr` (`/Game/Mods/PYTracker/Saves/TrackerSave.lastMap` _trackersave) _returnvalue)
      (`KismetArrayLibrary.Array_Clear` _s_trackerdatas)
      (set `/Game/Mods/PYTracker/Saves/TrackerSave.lastMap` _returnvalue _trackersave)
      (`self.SaveObjectToSlot` false))
    (`KismetArrayLibrary.Array_Add` _s_trackerdatas (`self.StrackerDummy`))
    (else
      (`KismetArrayLibrary.Array_Clear` _s_trackerdatas)
      (`KismetArrayLibrary.Array_Add` _s_trackerdatas (`self.StrackerDummy`))))
  (`self.SaveObjectToSlot` false))

(fn `SaveObjectToSlot`
  (params (isSaveToNewFile :type Boolean))
  (bind _trackersave (`self.TrackerSave`))
  (if isSaveToNewFile
    (`GameplayStatics.SaveGameToSlot` _trackersave (`KismetStringLibrary.Concat_StrStr` "_PYTracker_" (`self.AlternativeSaveFileName`)))
    (else
      (`GameplayStatics.SaveGameToSlot` _trackersave (`self.SaveGameName`)))))

(fn `SetAlternativeFileName`
  (params (Text :type Text))
  (bind (_returnvalue_year _returnvalue_month _returnvalue_day _returnvalue_hour _returnvalue_minute _returnvalue_second) (`KismetMathLibrary.BreakDateTime` (`KismetMathLibrary.Now`)))
  (bind _returnvalue (`GameplayStatics.GetCurrentLevelName` true))
  (set `self.AlternativeSaveFileName` (`KismetStringLibrary.Replace` (select `bool` (`KismetTextLibrary.TextIsEmpty` Text) :`false` (`KismetTextLibrary.Conv_TextToString` Text) :`true` (`KismetStringLibrary.Concat_StrStr` _returnvalue "_" (`KismetStringLibrary.Concat_StrStr` (`KismetStringLibrary.Conv_IntToString` _returnvalue_hour) "-" (`KismetStringLibrary.Conv_IntToString` _returnvalue_minute) "-" (`KismetStringLibrary.Conv_IntToString` _returnvalue_second) "_" (`KismetStringLibrary.Conv_IntToString` _returnvalue_day) "-" (`KismetStringLibrary.Conv_IntToString` _returnvalue_month)))) " ")))

(fn `UserConstructionScript`)