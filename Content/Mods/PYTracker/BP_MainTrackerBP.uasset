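; Mod actor that records the player's movement and replays saved tracks through a collisionless ghost character with its own material.
; BeginPlay creates BP_SaveGameManager and a hidden WBP_Menu.
; Each tick feeds player transform, velocity and level name to the manager, while stepping the dummy frame by frame through stored tracks in a loop.
; Rebindable keys toggle the menu, save tracks or write an alternate file; EndPlay can auto-save.
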(event `self.ReceiveBeginPlay`
  (`self.SpawnSaveManager`)
  (bind _returnvalue (`|GenericCreateObject` "/Game/Mods/PYTracker/WBP_Menu.WBP_Menu_C" self self))
  (`UserWidget.AddToViewport` _returnvalue 1)
  (`Widget.SetVisibility` _returnvalue "Collapsed")
  (set `self.WBP` _returnvalue))

(event `self.ReceiveTick`
  (params (DeltaSeconds :type "Float (single-precision)"))
  (bind _returnvalue (`GameplayStatics.GetPlayerCharacter` 0))
  (bind _indexarray (`self.IndexArray`))
  (bind _dummyplayer (`self.DummyPlayer`))
  (bind _s_trackerdatas (`/Game/Mods/PYTracker/Saves/TrackerSave.S_TrackerDatas` (`/Game/Mods/PYTracker/BP_SaveGameManager.TrackerSave` (`self.SaveGameManager`))))
  (bind (_transforms _velocity) (break `/Game/Mods/PYTracker/Saves/S_TrackerDataList` (`|GetArrayItem` _s_trackerdatas (`self.IndexArray`))))
  (`|ExecutionSequence`
    (:`then_0`
      (`self.CheckSaveToAnotherFile`)
      (`self.CheckMenuKeyPress`)
      (`self.CheckSaveTrackKeyPress`)
      (if (> (`KismetArrayLibrary.Array_Length` (`.Transforms_8_CAE2054046131B43AB9BB892CB85C7CD` (break `/Game/Mods/PYTracker/Saves/S_TrackerDataList` (`|GetArrayItem` (`/Game/Mods/PYTracker/Saves/TrackerSave.S_TrackerDatas` (`/Game/Mods/PYTracker/BP_SaveGameManager.TrackerSave` (`self.SaveGameManager`))))))) 10)
        (`|ExecutionSequence`
          (:`then_0`
            (`/Engine/EditorBlueprintResources/StandardMacros.DoOnce` false
              (:`Completed`
                (`self.SpawnDummy`))))
          (:`then_1`
            (`|ExecutionSequence`
              (:`then_0`
                (`self.K2_SetActorTransform` _dummyplayer (`|GetArrayItem` _transforms (`self.Index`)) false false)
                (set `MovementComponent.Velocity` (`|GetArrayItem` _velocity (stale _output_get)) (`self.GetComponentByClass` _dummyplayer "/Script/Engine.CharacterMovementComponent")))
              (:`then_1`
                (bind _result (`/Engine/EditorBlueprintResources/StandardMacros.IncrementInt` (`self.Index`))
                  (:`  `
                    (if (>= _result (`KismetArrayLibrary.Array_Length` _transforms))
                      (bind _output_get (set `self.Index` 0))
                      (`/Engine/EditorBlueprintResources/StandardMacros.IncrementInt` _indexarray
                        (:`  `
                          (if (>= _indexarray (`KismetArrayLibrary.Array_Length` _s_trackerdatas))
                            (set `self.IndexArray` 0)))))))))))))
    (:`then_1`
      (bind _returnvalue_2 (`GameplayStatics.GetCurrentLevelName` true))
      (`/Game/Mods/PYTracker/BP_SaveGameManager.AddToTrackerDummy` (`self.SaveGameManager`) (`self.GetTransform` _returnvalue) _returnvalue_2 (`self.GetVelocity` _returnvalue)))))

(event `self.ReceiveEndPlay`
  (params (EndPlayReason :type "EEndPlayReason Enum" :default "Destroyed"))
  (if (`/Game/Mods/PYTracker/Saves/TrackerSave.isAutoSaveOnRestart` (`/Game/Mods/PYTracker/BP_SaveGameManager.TrackerSave` (`self.SaveGameManager`)))
    (`/Game/Mods/PYTracker/BP_SaveGameManager.SaveCurrentTrack` (`self.SaveGameManager`))))

(fn `CheckMenuKeyPress`
  (bind _returnvalue (`GameplayStatics.GetPlayerController` 0))
  (bind _returnvalue_2 (`GameplayStatics.GetPlayerController` 0))
  (bind _wbp (`self.WBP`))
  (if (`PlayerController.WasInputKeyJustPressed` (`GameplayStatics.GetPlayerController` 0) (`BlueprintMapLibrary.Map_Find` (`/Game/Mods/PYTracker/Saves/TrackerSave.Binds` (`/Game/Mods/PYTracker/BP_SaveGameManager.TrackerSave` (`self.SaveGameManager`))) "NewEnumerator0"))
    (switch `ESlateVisibility` (`Widget.GetVisibility` _wbp)
      (:`Visible`
        (`Widget.SetVisibility` _wbp "Collapsed")
        (`WidgetBlueprintLibrary.SetInputMode_GameOnly` _returnvalue_2)
        (set `PlayerController.bShowMouseCursor` false _returnvalue))
      (:`Collapsed`
        (`Widget.SetVisibility` _wbp "Visible" :!label _label)
        (`WidgetBlueprintLibrary.SetInputMode_GameAndUIEx` _returnvalue_2 _wbp)
        (set `PlayerController.bShowMouseCursor` true _returnvalue))
      (:`Hidden`
        (goto _label)))))

(fn `CheckSaveToAnotherFile`
  (if (`PlayerController.WasInputKeyJustPressed` (`GameplayStatics.GetPlayerController` 0) (`BlueprintMapLibrary.Map_Find` (`/Game/Mods/PYTracker/Saves/TrackerSave.Binds` (`/Game/Mods/PYTracker/BP_SaveGameManager.TrackerSave` (`self.SaveGameManager`))) "NewEnumerator3"))
    (`/Game/Mods/PYTracker/BP_SaveGameManager.SetAlternativeFileName` (`self.SaveGameManager`) (`EditableTextBox.GetText` (`/Game/Mods/PYTracker/WBP_Menu.AltFileNamebox` (`self.WBP`))))
    (`/Game/Mods/PYTracker/BP_SaveGameManager.SaveObjectToSlot` (`self.SaveGameManager`) true)
    (`/Game/Mods/PYTracker/WBP_Menu.OnAltFileSaved` (`self.WBP`))))

(fn `CheckSaveTrackKeyPress`
  (if (`PlayerController.WasInputKeyJustPressed` (`GameplayStatics.GetPlayerController` 0) (`BlueprintMapLibrary.Map_Find` (`/Game/Mods/PYTracker/Saves/TrackerSave.Binds` (`/Game/Mods/PYTracker/BP_SaveGameManager.TrackerSave` (`self.SaveGameManager`))) "NewEnumerator2"))
    (`/Game/Mods/PYTracker/BP_SaveGameManager.SaveCurrentTrack` (`self.SaveGameManager`))
    (if (not (`/Game/Mods/PYTracker/Saves/TrackerSave.isResetArrayOnNewSave` (`/Game/Mods/PYTracker/BP_SaveGameManager.TrackerSave` (`self.SaveGameManager`))))
      (set `self.Index` 0)
      (set `self.IndexArray` 0))))

(fn `ModButtonWasPressed`
  (params (FunctionIndex :type Integer))
  (switch `int` FunctionIndex
    (:`0`
      (set `/Game/Mods/PYTracker/Saves/TrackerSave.Binds` (`|MakeMap` "NewEnumerator0" "Six" "NewEnumerator2" "MiddleMouseButton" "NewEnumerator3" :!type "/Game/Mods/PYTracker/Tracker_BindType Enum" :!valuetype "Key Structure") (`/Game/Mods/PYTracker/BP_SaveGameManager.TrackerSave` (`self.SaveGameManager`)))
      (`/Game/Mods/PYTracker/WBP_Menu.UpdateBinds` (`self.WBP`)))))

(fn `SpawnDummy`
  (bind _returnvalue (`|SpawnActorFromClass` "/Game/Game/BPCharacter_Demo.BPCharacter_Demo_C" (`KismetMathLibrary.MakeTransform` (`self.K2_GetActorLocation` (`GameplayStatics.GetPlayerCharacter` 0)) (struct) (1.0 1.0 1.0)) "AlwaysSpawn" "OverrideRootScale" null null))
  (`KismetArrayLibrary.Array_Add` (`Actor.Tags` _returnvalue) "Dummy")
  (bind _output_get (set `self.DummyPlayer` _returnvalue))
  (`self.SetActorEnableCollision` _output_get false)
  (`PrimitiveComponent.SetMaterial` (`self.GetComponentByClass` _output_get "/Script/Engine.SkeletalMeshComponent") 0 "/Game/Mods/PYTracker/DummyMaterial.DummyMaterial"))

(fn `SpawnSaveManager`
  (bind _returnvalue (`GameplayStatics.GetCurrentLevelName` true))
  (switch `string` _returnvalue
    (:`Default`
      (bind _returnvalue_2 (`|SpawnActorFromClass` "/Game/Mods/PYTracker/BP_SaveGameManager.BP_SaveGameManager_C" (`KismetMathLibrary.MakeTransform` (0.0 0.0 0.0)) "AlwaysSpawn" "OverrideRootScale" null self null))
      (set `self.SaveGameManager` _returnvalue_2))))

(fn `UserConstructionScript`
  (`parent.UserConstructionScript`))