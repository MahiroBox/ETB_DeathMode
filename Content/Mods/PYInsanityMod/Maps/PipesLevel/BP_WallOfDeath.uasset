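; Moving death wall for the Pipes level that kills any player character it overlaps and turns off the lights of pipes it touches.
; BeginPlay builds the wall at runtime as a replicated Actor with an added static mesh, attaching zero-scaled Portal and red glowstick actors.
; Tick moves the wall along DirectionToGo, dragging an oversized, pawn-ignoring Smiler at an offset, whose audio is relocated far away at spawn.
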(event `self.ReceiveBeginPlay`
  (`self.SpawnWall` (delegate `OnComponentBeginOverlap_Event_0`)))

(event `OnComponentBeginOverlap_Event_0`
  (params (OverlappedComponent :type "PrimitiveComponent Object Reference") (OtherActor :type "Actor Object Reference") (OtherComp :type "PrimitiveComponent Object Reference") (OtherBodyIndex :type Integer) (bFromSweep :type Boolean) (SweepResult :type "HitResult Structure (by ref)"))
  (bind _returnvalue (`GameplayStatics.GetObjectClass` OtherActor))
  (if (`KismetMathLibrary.ClassIsChildOf` _returnvalue "/Game/Game/BPCharacter_Demo.BPCharacter_Demo_C")
    (bind _asbpcharacter_demo (cast `/Game/Game/BPCharacter_Demo` OtherActor))
    (`/Game/Game/BPCharacter_Demo.KillClient` _asbpcharacter_demo)
    (`/Game/Game/BPCharacter_Demo.KillServer` _asbpcharacter_demo)
    (elif (`KismetMathLibrary.ClassIsChildOf` _returnvalue "/Game/Pipes/Pipe_On.Pipe_On_C")
      (bind _aspipe_on (cast `/Game/Pipes/Pipe_On` OtherActor))
      (`/Game/Pipes/Pipe_On.TurnOffLights` _aspipe_on))))

(event `self.ReceiveTick`
  (params (DeltaSeconds :type "Float (single-precision)"))
  (bind _returnvalue (`self.GetTransform` (`self.Wall`)))
  (`self.K2_AddActorWorldOffset` (`self.Wall`) (* (`self.DirectionToGo`) DeltaSeconds) false false)
  (`self.K2_SetActorTransform` (`self.Smiler`) (`KismetMathLibrary.MakeTransform` (`KismetMathLibrary.MakeVector` (.x (.location _returnvalue)) (+ (.y (.location _returnvalue)) -350.0) (+ (.z (.location _returnvalue)) -1000.0)) (.rotation _returnvalue)) false false))

(fn `SpawnWall`
  (params (Event :type "Delegate (by ref)"))
  (`|ExecutionSequence`
    (:`then_0`
      (bind _returnvalue (`|SpawnActorFromClass` "/Script/Engine.Actor" (`KismetMathLibrary.MakeTransform` (0.0 0.0 0.0)) "AlwaysSpawn" "OverrideRootScale" null null))
      (`self.SetReplicateMovement` _returnvalue true)
      (`self.SetReplicates` _returnvalue true)
      (bind _returnvalue_2 (`AddComponent|NODE_AddStaticMeshComponent-1` :`self` _returnvalue))
      (`ActorComponent.SetIsReplicated` _returnvalue_2 true)
      (add `PrimitiveComponent.OnComponentBeginOverlap` _returnvalue_2 Event)
      (bind _returnvalue_3 (`|SpawnActorFromClass` "/Game/Core/Portal.Portal_C" (`KismetMathLibrary.MakeTransform` (0.0 0.0 0.0)) "AlwaysSpawn" "OverrideRootScale" null null))
      (`self.K2_AttachToActor` _returnvalue_3 _returnvalue "None" "SnapToTarget" "SnapToTarget" "SnapToTarget" true)
      (bind _defaultsceneroot (`/Game/Game/BP_ExitZone.DefaultSceneRoot` _returnvalue_3))
      (`ActorComponent.SetIsReplicated` _defaultsceneroot true)
      (`SceneComponent.K2_SetRelativeTransform` _defaultsceneroot (`KismetMathLibrary.MakeTransform` (163.610001 0.0 50.0) (struct) (0.0 0.0 0.0)) false false))
    (:`then_1`
      (`self.K2_SetActorTransform` _returnvalue (`self.GetTransform`) false false)
      (bind _output_get (set `self.Wall` _returnvalue))
      (bind _returnvalue_4 (`|SpawnActorFromClass` "/Game/NewInventorySystem/Items/BP_Item_Glowstick_Red.BP_Item_Glowstick_Red_C" (`KismetMathLibrary.MakeTransform` (0.0 0.0 0.0)) "AlwaysSpawn" "OverrideRootScale" null null))
      (`self.K2_AttachToActor` _returnvalue_4 _output_get "None" "SnapToTarget" "SnapToTarget" "SnapToTarget" true)
      (`SceneComponent.K2_SetRelativeTransform` (`Actor.RootComponent` _returnvalue_4) (`KismetMathLibrary.MakeTransform` (163.610001 0.0 50.0) (struct) (0.0 0.0 0.0)) false false)
      (bind _returnvalue_5 (`|SpawnActorFromClass` "/Game/Entity/Smiler_BP.Smiler_BP_C" (`KismetMathLibrary.MakeTransform` (0.0 0.0 0.0)) "AlwaysSpawn" "OverrideRootScale" null null))
      (bind _output_get_2 (set `self.Smiler` _returnvalue_5))
      (bind _returnvalue_6 (`self.K2_GetComponentsByClass` _returnvalue_5 "/Script/Engine.PrimitiveComponent"))
      (`PrimitiveComponent.SetCollisionResponseToChannel` _returnvalue_6 "ECC_Pawn" "ECR_Ignore")
      (`SceneComponent.SetWorldScale3D` _returnvalue_6 (300.0 5.0 10000.0))
      (`ActorComponent.SetIsReplicated` (`self.K2_GetComponentsByClass` _output_get_2 "/Script/Engine.ActorComponent") true)
      (`SceneComponent.K2_SetWorldLocation` (`self.K2_GetComponentsByClass` _output_get_2 "/Script/Engine.AudioComponent") (0.0 0.0 100000.0) false false))))

(fn `UserConstructionScript`)