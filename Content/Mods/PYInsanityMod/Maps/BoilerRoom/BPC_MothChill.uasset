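; Actor component for the BoilerRoom map in PYInsanityMod that modifies its owning BP_Moth, apparently to calm it down.
; On BeginPlay it moves all of the moth's audio components far below their parent and destroys Audio and Audio1.
; Every tick it overwrites the moth's StartTransform with its current transform, so that stored start point follows the moth.
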(event `self.ReceiveBeginPlay`
  (bind _asbp_moth (cast `/Game/Entity/DeathMoth/FemaleMoth/BP_Moth` (`self.GetOwner`)))
  (bind _output_get (set `self.Moth` _asbp_moth))
  (for _array_element (`Actor.K2_GetComponentsByClass` _output_get "/Script/Engine.AudioComponent")
    (`SceneComponent.K2_SetRelativeLocation` _array_element (0.0 0.0 -10000.0) false false))
  (`self.K2_DestroyComponent` (`/Game/Entity/DeathMoth/FemaleMoth/BP_Moth.Audio` _output_get))
  (`self.K2_DestroyComponent` (`/Game/Entity/DeathMoth/FemaleMoth/BP_Moth.Audio1` _output_get)))

(event `self.ReceiveTick`
  (params (DeltaSeconds :type "Float (single-precision)"))
  (bind _moth (`self.Moth`))
  (set `/Game/Entity/DeathMoth/FemaleMoth/BP_Moth.StartTransform` (`Actor.GetTransform` _moth) _moth))