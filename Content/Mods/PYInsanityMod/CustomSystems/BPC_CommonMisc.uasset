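; BPC_CommonMisc is an actor component that adds optional utility behaviors to its owner, most switched off by a -1 value.
; On BeginPlay it can pause the owner's overlap events, teleport it after a delay, attach a spawned or referenced actor, and destroy it after a delay.
; For Character owners, it caches the default walk speed and reapplies a custom absolute or multiplied speed every Tick.
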(event `self.ReceiveBeginPlay`
  (bind _delaytodeleteowner (`self.DelayToDeleteOwner`))
  (bind _attachactor (`self.AttachActor`))
  (`self.GetActor`)
  (`|ExecutionSequence`
    (:`then_0`
      (`self.DisableColl`))
    (:`then_1`
      (`self.SetTransform`))
    (:`then_2`
      (`self.GetSpeed`))
    (:`then_3`
      (if (`KismetSystemLibrary.IsValidClass` _attachactor)
        (bind _returnvalue (`|SpawnActorFromClass` _attachactor (`KismetMathLibrary.MakeTransform` (0.0 0.0 0.0)) "AlwaysSpawn" "OverrideRootScale" null null))
        (`Actor.K2_AttachToActor` _returnvalue (`self.OwnerActor`) "None" "SnapToTarget" "SnapToTarget" "SnapToTarget" true)
        (else
          (`Actor.K2_AttachToActor` (`self.AttachRefActorToOwner`) (`self.OwnerActor`) "None" "KeepRelative" "KeepRelative" "KeepRelative" true))))
    (:`then_4`
      (if (not (== _delaytodeleteowner -1.0))
        (`KismetSystemLibrary.Delay` _delaytodeleteowner)
        (`Actor.K2_DestroyActor` (`self.OwnerActor`))))))

(event `self.ReceiveTick`
  (params (DeltaSeconds :type "Float (single-precision)"))
  (bind _customspeed (`self.CustomSpeed`))
  (if (not (== _customspeed -1.0))
    (set `CharacterMovementComponent.MaxWalkSpeed` (select `bool` (`self.isMultiplySpeed`) :`false` _customspeed :`true` (* (`self.defaultSpeed`) (`self.CustomSpeed`))) (`Character.CharacterMovement` (`self.As Character`)))))

(fn `GetActor`
  (set `self.OwnerActor` (`self.GetOwner`)))

(fn `GetPrimitives`
  (for _array_element (`Actor.K2_GetComponentsByClass` (`self.OwnerActor`) "/Script/Engine.PrimitiveComponent")
    (`KismetArrayLibrary.Array_Add` (`self.Primitives`) _array_element)))