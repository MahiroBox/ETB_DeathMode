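; BPC_AISpeed is an actor component in PYInsanityMod that overrides the walk speed of its owning Character, presumably an AI.
; BeginPlay records MaxWalkSpeed as DefaultSpeed, reading it through the Character reference before that reference is assigned from a cast of the owner.
; Every Tick rewrites MaxWalkSpeed to Speed, or to DefaultSpeed plus Speed when IsAddToCurrentSpeed is set.
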(event `self.ReceiveBeginPlay`
  (set `self.defaultSpeed` (`CharacterMovementComponent.MaxWalkSpeed` (`Character.CharacterMovement` (`self.Character`))))
  (bind _ascharacter (cast `Character` (`self.GetOwner`)))
  (set `self.Character` _ascharacter))

(event `self.ReceiveTick`
  (params (DeltaSeconds :type "Float (single-precision)"))
  (set `CharacterMovementComponent.MaxWalkSpeed` (select `bool` (`self.isAddToCurrentSpeed`) :`false` (`self.Speed`) :`true` (+ (`self.defaultSpeed`) (`self.Speed`))) (`Character.CharacterMovement` (`self.Character`))))