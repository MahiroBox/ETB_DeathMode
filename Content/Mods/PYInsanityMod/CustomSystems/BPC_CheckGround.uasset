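; Actor component that switches its owning Character between Walking and Flying movement based on whether ground is beneath it.
; While enabled, each tick runs a Camera-channel line trace down the character's local up axis, ignoring the character.
; A pair of DoOnce gates that reset each other limits movement mode changes and OnStateChanged broadcasts to ground/air transitions.
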(event `self.ReceiveBeginPlay`
  (bind _ascharacter (cast `Character` (`self.GetOwner`)))
  (set `self.Character` _ascharacter))

(event `self.ReceiveTick`
  (params (DeltaSeconds :type "Float (single-precision)"))
  (bind _character (`self.Character`))
  (bind _character_2 (`self.Character`))
  (bind _returnvalue_location (`KismetMathLibrary.BreakTransform` (`Actor.GetTransform` _character)))
  (bind _charactermovement (`Character.CharacterMovement` (`self.Character`)))
  (if (not (`self.isDisabled`))
    (bind (_outhit _returnvalue) (`KismetSystemLibrary.LineTraceSingle` _returnvalue_location (+ _returnvalue_location (* (`Actor.GetActorUpVector` _character) -230.0)) "TraceTypeQuery2" false (`|MakeArray` _character :!type "Actor Object Reference")))
    (if _returnvalue
      (`|ExecutionSequence`
        (:`then_0`
          (`/Engine/EditorBlueprintResources/StandardMacros.DoOnce` true :!label _label
            (:`Completed`
              (`CharacterMovementComponent.SetMovementMode` _charactermovement "MOVE_Walking" 0)
              (`self.OnStateChanged` true _character_2 self))))
        (:`then_1`
          (goto _label_2 :!via `Reset`)))
      (else
        (`|ExecutionSequence`
          (:`then_0`
            (`/Engine/EditorBlueprintResources/StandardMacros.DoOnce` false :!label _label_2
              (:`Completed`
                (`CharacterMovementComponent.SetMovementMode` _charactermovement "MOVE_Flying" 0)
                (`self.OnStateChanged` false _character_2 self))))
          (:`then_1`
            (goto _label :!via `Reset`)))))))