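; Actor component that briefly teleports its owning Character onto the player at BeginPlay, apparently to activate a moth entity, then destroys itself.
; It hides the owner, ignores Pawn collision on its primitives and stops AI movement.
; After a short delay, it restores location and visibility.
; Pawn collision is restored from saved responses, though these are read from the WorldStatic channel rather than Pawn.
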(event `self.ReceiveBeginPlay`
  (bind _ascharacter (cast `Character` (`self.GetOwner`)))
  (set `self.Char` _ascharacter)
  (`self.DoTrigger`
    (:`exec`
      (`self.K2_DestroyComponent`))))