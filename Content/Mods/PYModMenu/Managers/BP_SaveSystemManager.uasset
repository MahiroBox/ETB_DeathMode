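; Save manager for the PY Mod Menu that persists key bindings in an OB_PYMM_Saves save game object.
; On BeginPlay it loads or creates the save in its SlotName slot, then deletes any save in the hardcoded "PYModMenuSaves" slot.
; SetKeyBind writes a key into the SBinds map by type and saves immediately, while FindKeyByEnum reads bindings back from the cached object.
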(event `self.ReceiveBeginPlay`
  (`|ExecutionSequence`
    (:`then_0`
      (bind _returnvalue (`GameplayStatics.DoesSaveGameExist` (`self.SlotName`)))
      (if _returnvalue
        (bind _returnvalue_2 (`GameplayStatics.LoadGameFromSlot` (`self.SlotName`)))
        (bind _asob_pymm_saves (cast `/Game/Mods/PYModMenu/SaveSystem/OB_PYMM_Saves` _returnvalue_2))
        (set `self.SavesOB` _asob_pymm_saves)
        (else
          (bind _returnvalue_3 (`GameplayStatics.CreateSaveGameObject` "/Game/Mods/PYModMenu/SaveSystem/OB_PYMM_Saves.OB_PYMM_Saves_C"))
          (`GameplayStatics.SaveGameToSlot` _returnvalue_3 (`self.SlotName`))
          (set `self.SavesOB` _returnvalue_3))))
    (:`then_1`
      (bind _returnvalue_4 (`GameplayStatics.DoesSaveGameExist` "PYModMenuSaves"))
      (if _returnvalue_4
        (`GameplayStatics.DeleteGameInSlot` "PYModMenuSaves")))))

(fn `FindKeyByEnum`
  (params (Key :type "/Game/Mods/PYModMenu/SaveSystem/BindType Enum" :default "NewEnumerator0"))
  (returns (Value :type "Key Structure"))
  (return (`BlueprintMapLibrary.Map_Find` (`/Game/Mods/PYModMenu/SaveSystem/OB_PYMM_Saves.SBinds` (`self.SavesOB`)) Key)))

(fn `SaveSlot`
  (`GameplayStatics.SaveGameToSlot` (`self.SavesOB`) (`self.SlotName`)))

(fn `SetKeyBind`
  (params (`New Key` :type "Key Structure" :default "None") (Type :type "/Game/Mods/PYModMenu/SaveSystem/BindType Enum" :default "NewEnumerator0"))
  (`BlueprintMapLibrary.Map_Add` (`/Game/Mods/PYModMenu/SaveSystem/OB_PYMM_Saves.SBinds` (`self.SavesOB`)) Type `New Key`)
  (`self.SaveSlot`))

(fn `UserConstructionScript`)