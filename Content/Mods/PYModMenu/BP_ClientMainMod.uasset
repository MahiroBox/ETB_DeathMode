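; Client-side actor for the PYModMenu mod, apparently meant to register players who have the mod installed.
; On BeginPlay or a CallToserver event it calls the add-player-with-mod event.
; That event only prints debug text and the name of player character 0, ignoring its Player input.
; The node that would add to the main Blueprint's PlayersWithMod list is disconnected, so no registration occurs.
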(event `CallToserver`
  (`self.SR_AddPlayerWithMod` null))

(event `self.ReceiveBeginPlay`
  (`/Game/Mods/Z_DebugLog_P/BlueprintLibraries/BFL_DebugLog.ModPrint` "ClientMainModActor")
  (`self.SR_AddPlayerWithMod` null))

(event `SR_AddPlayerWithMod`
  (params (Player :type "PlayerController Object Reference"))
  (`/Game/Mods/Z_DebugLog_P/BlueprintLibraries/BFL_DebugLog.ModPrint` "CALLED")
  (`/Game/Mods/Z_DebugLog_P/BlueprintLibraries/BFL_DebugLog.ModPrint` (`PlayerState.GetPlayerName` (`Pawn.PlayerState` (`GameplayStatics.GetPlayerCharacter` 0)))))

(fn `UserConstructionScript`)