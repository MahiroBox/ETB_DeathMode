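; Entity randomizer mod actor that, when the host presses Z, swaps every non-player Character for a different entity type at the same transform.
; It saves each transform, destroys the entity, reshuffles the class list until the first entry differs, then spawns that class.
; A server-only widget reports status.
; About every second, the server also moves non-player primitives to the Vehicle channel and ignores it, so they pass through each other.
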(event `self.ReceiveBeginPlay`
  (if (`KismetSystemLibrary.IsServer`)
    (`self.SpawnWidgetInGame`)))

(event `self.ReceiveTick`
  (params (DeltaSeconds :type "Float (single-precision)"))
  ;[0 1 0.2031 1 16] Initial Operation
  (if (`KismetSystemLibrary.IsServer`)
    (`|ExecutionSequence`
      (:`then_0`
        (`KismetSystemLibrary.Delay` 1.0)
        (bind _outactors (`GameplayStatics.GetAllActorsOfClass` "/Script/Engine.Character"))
        (for _array_element _outactors
          (if (not (`KismetMathLibrary.ClassIsChildOf` (`GameplayStatics.GetObjectClass` _array_element) "/Game/Game/BPCharacter_Demo.BPCharacter_Demo_C"))
            (for _array_element_2 (`self.K2_GetComponentsByClass` _array_element "/Script/Engine.PrimitiveComponent")
              (`PrimitiveComponent.SetCollisionResponseToChannel` _array_element_2 "ECC_Vehicle" "ECR_Ignore")
              (`PrimitiveComponent.SetCollisionObjectType` _array_element_2 "ECC_Vehicle")))))
      (:`then_1`
        (if (`PlayerController.WasInputKeyJustPressed` (`GameplayStatics.GetPlayerController` 0) "Z")
          ;[0 0.3437 1 1 16] Gets all Entities And Randomize After Input
          (`self.Get And Set Entities`))))))

(fn `ModButtonWasPressed`
  (params (FunctionIndex :type Integer))
  (switch `int` FunctionIndex))

(fn `SpawnWidgetInGame`
  (bind _wbp_erandomwidget (`self.WBP_ERandomWidget`))
  (bind _returnvalue (`GameplayStatics.GetCurrentLevelName` true))
  (switch `string` _returnvalue
    (:`Default`
      (bind _returnvalue_2 (`|GenericCreateObject` "/Game/Mods/PYEntityRandomizer/WBP_ERandom.WBP_ERandom_C" self))
      (bind _output_get (set `self.WBP_ERandomWidget` _returnvalue_2))
      (`UserWidget.AddToViewport` _output_get 1)
      (`/Game/Mods/PYEntityRandomizer/WBP_ERandom.SetText` _wbp_erandomwidget (`/Game/Mods/PYEntityRandomizer/WBP_ERandom.Remember` _wbp_erandomwidget)))))

(fn `UserConstructionScript`
  (`parent.UserConstructionScript`))