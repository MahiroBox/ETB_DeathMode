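; First-person character Blueprint that appears to test client-side actor spawning and events in multiplayer.
; On Tick, a non-server instance polls the F key and calls Func.
; Func spawns a ClientActor owned by the character and caches it as Cube, or calls ClientActorEvent on it if already valid.
; The HasSpawn RepNotify only prints a debug string.
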(event `self.ReceiveTick`
  (params (DeltaSeconds :type "Float (single-precision)"))
  (if (`KismetSystemLibrary.IsServer`)
    _
    (elif (`PlayerController.WasInputKeyJustPressed` (`GameplayStatics.GetPlayerController` 0) "F")
      (`self.Func`))))

(event `Func`
  (`/Engine/EditorBlueprintResources/StandardMacros.IsValid` (`self.Cube`)
    (:`Is Valid`
      (`/Game/_DefaultMap/ClientActor.ClientActor_Event` (`self.Cube`)))
    (:`Is Not Valid`
      (bind _returnvalue (`|SpawnActorFromClass` "/Game/_DefaultMap/ClientActor.ClientActor_C" (`KismetMathLibrary.MakeTransform` (0.0 0.0 0.0)) "AlwaysSpawn" "OverrideRootScale" self self null))
      (set `self.Cube` _returnvalue))))

(fn `OnRep_HasSpawn`
  (`KismetSystemLibrary.PrintString` "2"))

(fn `UserConstructionScript`)